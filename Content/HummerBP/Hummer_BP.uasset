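; Throwable hammer ("Hummer") actor that the first-person player can throw and recall.
; ThrowHummer rotates it and flies it along the given direction at constant speed on Tick, without sweeping.
; MoveToPlayer recalls it when the player lacks it and is not overlapping it, interpolating location (swept) and rotation toward the player.
; CollisionBox overlap during recall disables HardBox collision and calls TakeHummer on the character.
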(event OnComponentBeginOverlap(collisionBox)
  (params (OverlappedComponent :type Primitive%20Component%20Object%20Reference) (OtherActor :type Actor%20Object%20Reference) (OtherComp :type Primitive%20Component%20Object%20Reference) (OtherBodyIndex :type Integer) (bFromSweep :type Boolean) (SweepResult :type Hit%20Result%20Structure%20%28by%20ref%29))
  (bind _asfirst_person_character (Utilities|Casting|CastToFirstPersonCharacter OtherActor))
  (if (Variables|Default|GetMovingToPlayer)
    (Variables|Default|SetMovingToPlayer false)
    (Collision|SetCollisionEnabled (Variables|Default|GethardBox) "NoCollision")
    (Default|TakeHummer _asfirst_person_character)))

(event EventBeginPlay)

(event EventTick
  (params (DeltaSeconds :type Float%20%28single-precision%29))
  (bind _player (Variables|Default|Getplayer))
  (Utilities|FlowControl|Sequence
    (:then_0
      (if (Variables|Default|GetMovingToPlayer)
        (Transformation|SetActorLocation (Math|Interpolation|VInterpTo (Transformation|GetActorLocation) (Transformation|GetActorLocation _player) DeltaSeconds 11.0) true false)
        (Transformation|SetActorRotation (Math|Interpolation|RInterpTo (Transformation|GetActorRotation) (Transformation|GetActorRotation _player) DeltaSeconds 11.0))))
    (:then_1
      (if (Variables|Default|GetisThrowing)
        (Transformation|AddActorWorldOffset (* (* (Variables|Default|GetThrowingDirection) DeltaSeconds) 5e+03))))))

(fn ConstructionScript)

(fn MovetoPlayer
  (if (not (Collision|IsOverlappingActor (Variables|Default|GetcollisionBox) (Variables|Default|Getplayer) :!class /Script/Engine.PrimitiveComponent))
    (bind _asfirst_person_character (Utilities|Casting|CastToFirstPersonCharacter (Variables|Default|Getplayer)))
    (if (not (Variables|/Game/FirstPersonBP/Blueprints/FirstPersonCharacter.FirstPersonCharacter_C|GethaveHummer _asfirst_person_character))
      (Collision|SetCollisionEnabled (Variables|Default|GethardBox) "QueryAndPhysics")
      (Variables|Default|SetMovingToPlayer true)
      (Variables|Default|SetisThrowing false))))

(fn ThrowHummer
  (params (Direction :type Vector))
  (Variables|Default|SetThrowingDirection Direction)
  (Variables|Default|SetisThrowing true)
  (Variables|Default|SetMovingToPlayer false)
  (Collision|SetCollisionEnabled (Variables|Default|GethardBox) "QueryAndPhysics")
  (Transformation|AddActorLocalRotation "-90.000000, 0, 0" false false))