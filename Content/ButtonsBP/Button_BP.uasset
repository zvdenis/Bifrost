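; One-shot pressure button that opens its linked Door when something overlaps or hits its Box trigger.
; The first trigger sets IsPressed to block repeats, plays a stone-sliding 2D sound, opens the Door if the reference check passes and prints a debug message.
; A timeline then moves the Cube along a Spline, sampling its location from the ButtonTime track scaled by Distance.
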(event OnComponentBeginOverlap(Box)
  (params (OverlappedComponent :type Primitive%20Component%20Object%20Reference) (OtherActor :type Actor%20Object%20Reference) (OtherComp :type Primitive%20Component%20Object%20Reference) (OtherBodyIndex :type Integer) (bFromSweep :type Boolean) (SweepResult :type Hit%20Result%20Structure%20%28by%20ref%29))
  (bind _door (Variables|Default|Getdoor))
  (if (not (Variables|Default|GetisPressed))
    (Audio|SpawnSound2D "/Game/ButtonsBP/Камень_двигают_по_другому_камню__mp3cut_net_.Камень_двигают_по_другому_камню__mp3cut_net_" 1.0 1.0 0.0 0)
    (Variables|Default|SetisPressed true)
    (if (== _door 0)
      _
      (else
        (Default|Open _door)))
    (Development|PrintString "Button pressed")
    (Components|Timeline|SetPlayRate (Variables|Default|GetTimeline_0) 1.0)
    (bind _buttontime (Timeline|Timeline_0 Play)
      (:Update
        (Transformation|SetWorldLocation (Variables|Default|GetCube) (Spline|GetLocationatTime (Variables|Default|GetSpline) (* _buttontime (Variables|Default|Getdistance)) "World" false) false false)))))

(event OnComponentHit(Box)
  (params (HitComponent :type Primitive%20Component%20Object%20Reference) (OtherActor :type Actor%20Object%20Reference) (OtherComp :type Primitive%20Component%20Object%20Reference) (NormalImpulse :type Vector :default "0, 0, 0") (Hit :type Hit%20Result%20Structure%20%28by%20ref%29))
  (bind _door (Variables|Default|Getdoor))
  (if (not (Variables|Default|GetisPressed))
    (Audio|SpawnSound2D "/Game/ButtonsBP/Камень_двигают_по_другому_камню__mp3cut_net_.Камень_двигают_по_другому_камню__mp3cut_net_" 1.0 1.0 0.0 0)
    (Variables|Default|SetisPressed true)
    (if (== _door 0)
      _
      (else
        (Default|Open _door)))
    (Development|PrintString "Button pressed")
    (Components|Timeline|SetPlayRate (Variables|Default|GetTimeline_0) 1.0)
    (bind _buttontime (Timeline|Timeline_0 Play)
      (:Update
        (Transformation|SetWorldLocation (Variables|Default|GetCube) (Spline|GetLocationatTime (Variables|Default|GetSpline) (* _buttontime (Variables|Default|Getdistance)) "World" false) false false)))))

(event EventTick
  (params (DeltaSeconds :type Float%20%28single-precision%29)))

(fn ConstructionScript)