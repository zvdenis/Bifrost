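; FoldingDoor_BP is an activated door that opens once, sliding two cube panels along their own splines.
; The Open event checks and sets IsOpened, then plays a timeline.
; Each update multiplies the timeline value by Distance to sample both splines and place the panels in world space without sweeping.
; The graph has no closing logic.
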(event EventBeginPlay)

(event Collision|EventActorBeginOverlap
  (params (OtherActor :type Actor%20Object%20Reference))
  (|CallParentFunction OtherActor) ; This node is disabled and will not be called.\nDrag off pins to build functionality.
)

(event EventTick
  (params (DeltaSeconds :type Float%20%28single-precision%29))
  (|CallParentFunction DeltaSeconds) ; This node is disabled and will not be called.\nDrag off pins to build functionality.
)

(event EventOpen
  (|CallParentFunction)
  (if (not (Variables|Default|GetisOpened))
    (Variables|Default|SetisOpened true)
    (bind _buttontime (Timeline|Timeline_0 Play)
      (:Update
        (Transformation|SetWorldLocation (Variables|Default|GetCube) (Spline|GetLocationatTime (Variables|Default|GetSpline) (* _buttontime (Variables|Default|Getdistance)) "World" false) false false)
        (Transformation|SetWorldLocation (Variables|Default|GetCube1) (Spline|GetLocationatTime (Variables|Default|GetSpline1) (* _buttontime (Variables|Default|Getdistance)) "World" false) false false)))))

(fn ConstructionScript
  (|CallParentFunction))